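; Worker actor that autonomously hauls crates to trucks until the player's TwinStickPawn signals loading to stop.
; Starting after a short BeginPlay delay, it loops: claims the nearest free crate, glides to it at distance-scaled duration, destroys it, then carries the load to an assigned truck.
; The truck's loaded count increments before arrival, and the pawn's crates-to-load count decrements each trip.
; Once loading stops, it decrements the pawn's workers-to-mount count and destroys itself.
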(event EventBeginPlay
  (Utilities|FlowControl|Delay 2.0)
  (bind _astwin_stick_pawn (Utilities|Casting|CastToTwinStickPawn (Game|Player|GetPlayerPawn 0) :!label _label))
  (if (Variables|/Game/TwinStickBP/Blueprints/TwinStickPawn.TwinStickPawn_C|GetStopLoading _astwin_stick_pawn) ; if time for loading passed
    (Math|Integer|DecrementInt (Variables|/Game/TwinStickBP/Blueprints/TwinStickPawn.TwinStickPawn_C|GetWorkersToMount _astwin_stick_pawn)
      (:%20%20
        (Actor|DestroyActor) ; Destroy actor when truck boarded
      ))
    (else
      (Math|Integer|DecrementInt (Variables|/Game/TwinStickBP/Blueprints/TwinStickPawn.TwinStickPawn_C|GetLocal_CratesToLoad _astwin_stick_pawn)
        (:%20%20
          (bind (_nearestactor _distanceofnearestactor) (CallFunction|FindNearestCrate (Transformation|GetActorLocation) :!label _label_2))
          (bind _asbp_crate (Utilities|Casting|CastToBP_Crate _nearestactor))
          (if (Variables|/Game/MyBlueprint/BP_Crate.BP_Crate_C|GetLocal_IsBeingLoaded _asbp_crate) ; check if crate is not already being loaded
            (goto _label_2)
            (else
              (Variables|/Game/MyBlueprint/BP_Crate.BP_Crate_C|SetLocal_IsBeingLoaded _asbp_crate true)
              (Components|MoveComponentTo (Variables|Transformation|GetRootComponent) (Transformation|GetActorLocation _nearestactor) "0, 0, 0" true true (/ _distanceofnearestactor 2e+02) false) ; move to nearest crate
              (Actor|DestroyActor _nearestactor)
              (Variables|Default|SetHasCrate true) ; Mark that worker has a crate
              (bind _leastloadedtruck (CallFunction|AssignLoadtoTruck))
              ;[1 1 1] Increment crates loaded counter in selected truck
              (bind _asbp_truck (Utilities|Casting|CastToBP_Truck _leastloadedtruck))
              (Math|Integer|IncrementInt (Variables|/Game/MyBlueprint/BP_Truck.BP_Truck_C|GetLocal_CratesLoaded _asbp_truck)
                (:%20%20
                  (Components|MoveComponentTo (Variables|Transformation|GetRootComponent) (Transformation|GetActorLocation _leastloadedtruck) "0, 0, 0" true true 2.0 false) ; move to truck
                  (Variables|Default|SetHasCrate false) ; Mark worker that he has crate no more
                  (Utilities|FlowControl|Delay 0.5)
                  (goto _label))))))))))

(event Collision|EventActorBeginOverlap
  (params (OtherActor :type Actor%20Object%20Reference)))

(event EventTick
  (params (DeltaSeconds :type Float%20%28single-precision%29)))

(fn ConstructionScript)