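; BP_ScaredWorker is a worker actor that, when ScaredBegin fires, either flees the player or boards a truck after a short delay.
; LocalRunAway selects the branch: fleeing moves the root along a vector from GetVectorToPlayerPawn, while mounting eases it to one of the first three BP_Truck actors at random.
; Both branches decrement WorkersToMount on the TwinStickPawn, and only the mounting worker destroys itself afterwards.
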(event Custom|Event%20ScaredBegin
  (Utilities|FlowControl|Delay 0.5)
  (if (Variables|Default|GetLocal_RunAway) ; true to run away and false for mounting trucks
    ;[1 1 1] Running away from player pawn
    (bind _astwin_stick_pawn (Utilities|Casting|CastToTwinStickPawn (Game|Player|GetPlayerPawn 0)))
    (Math|Integer|DecrementInt (Variables|/Game/TwinStickBP/Blueprints/TwinStickPawn.TwinStickPawn_C|GetWorkersToMount _astwin_stick_pawn)
      (:%20%20
        (bind _vector (CallFunction|GetVectortoPlayerPawn (Game|Player|GetPlayerPawn 0) self))
        (Components|MoveComponentTo (Variables|Transformation|GetRootComponent self) _vector "0, 0, 0" false true 5.0 false)
        (Development|PrintString "Worker ran")))
    (else
      ;[1 1 1] mounting the trucks
      (bind _outactors (Actor|GetAllActorsOfClass "/Game/MyBlueprint/BP_Truck.BP_Truck_C"))
      (Components|MoveComponentTo (Variables|Transformation|GetRootComponent self) (Transformation|GetActorLocation (Utilities|Array|Get(acopy) _outactors (Math|Random|RandomInteger 3))) "0, 0, 0" true true 3.0 false)
      (bind _astwin_stick_pawn_2 (Utilities|Casting|CastToTwinStickPawn (Game|Player|GetPlayerPawn 0)))
      (Math|Integer|DecrementInt (Variables|/Game/TwinStickBP/Blueprints/TwinStickPawn.TwinStickPawn_C|GetWorkersToMount _astwin_stick_pawn_2)
        (:%20%20
          (Actor|DestroyActor))))))

(fn ConstructionScript)