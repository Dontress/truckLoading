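; Blueprint function library of gameplay helpers for crate loading and for workers fleeing the player.
; FindNearestCrate scans all crates for the closest one not already being loaded, while AssignLoadToTruck scans all trucks for the least loaded.
; GetVectorToPlayerPawn projects a flee point from the player through the scared worker at a fixed distance, keeping the worker's height, and prints a debug string.
; InvertBool returns the negated input.
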(fn FindNearestCrate
  (params (TargetLocation :type Vector))
  (bind _outactors (Actor|GetAllActorsOfClass 0 "/Game/MyBlueprint/BP_Crate.BP_Crate_C"))
  (for _array_element _outactors
    (if (< (Math|Vector|Distance(Vector) (Transformation|GetActorLocation _array_element) TargetLocation) (LocalVariables|GetLocal_NearestValue))
      (bind _asbp_crate (Utilities|Casting|CastToBP_Crate _array_element))
      (if (not (Variables|/Game/MyBlueprint/BP_Crate.BP_Crate_C|GetLocal_IsBeingLoaded _asbp_crate))
        (LocalVariables|SetLocal_NearestValue (Math|Vector|Distance(Vector) (Transformation|GetActorLocation _array_element) TargetLocation))
        (LocalVariables|SetLocal_NearestActor _array_element))))
  (return (LocalVariables|GetLocal_NearestActor) (LocalVariables|GetLocal_NearestValue)))

(fn AssignLoadtoTruck
  (bind _outactors (Actor|GetAllActorsOfClass 0 "/Game/MyBlueprint/BP_Truck.BP_Truck_C"))
  (for _array_element _outactors
    (if (<= (Variables|/Game/MyBlueprint/BP_Truck.BP_Truck_C|GetLocal_CratesLoaded _array_element) (LocalVariables|GetLocalLib_CratesLoaded))
      (LocalVariables|SetLocal_LeastLoadedTruck _array_element)
      (LocalVariables|SetLocalLib_CratesLoaded (Variables|/Game/MyBlueprint/BP_Truck.BP_Truck_C|GetLocal_CratesLoaded _array_element))))
  (return (LocalVariables|GetLocal_LeastLoadedTruck)))

(fn InvertBool
  (params (InputBool :type Boolean))
  (if InputBool
    (LocalVariables|SetLocal_boolVal false)
    (else
      (LocalVariables|SetLocal_boolVal true)))
  (return (LocalVariables|GetLocal_boolVal)))

(fn GetVectortoPlayerPawn
  (params (PlayerPawn :type Actor%20Object%20Reference) (ActorToRun :type Actor%20Object%20Reference))
  (bind _returnvalue (Transformation|GetActorLocation ActorToRun))
  (bind _returnvalue_2 (Transformation|GetActorLocation PlayerPawn))
  (bind _returnvalue_3 (Math|Rotator|FindLookatRotation _returnvalue _returnvalue_2))
  (bind _returnvalue_4 (Math|Vector|GetForwardVector _returnvalue_3))
  (bind _returnvalue_5 (* _returnvalue_4 -4e+03))
  (bind _returnvalue_6 (+ _returnvalue_2 _returnvalue_5))
  (bind (_x _y) (Math|Vector|BreakVector _returnvalue_6))
  (Development|PrintString 0 "Hello" true true "(R=0.000000,G=0.660000,B=1.000000,A=1.000000)" 2e+01)
  (return (Math|Vector|MakeVector _x _y (.Z (Math|Vector|BreakVector _returnvalue)))))